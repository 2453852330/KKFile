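; BP_Example is an example Blueprint that exercises KK-prefixed file utility functions and prints the results.
; On BeginPlay, a sequence builds and stores a path to a text file in the project's Saved directory, then reports whether that file exists.
; It then writes a test string to the file, reloads it as a string array and prints the write result and array length.
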(event EventBeginPlay
  (bind _returnvalue (Class|KKFileBlueprintFunctionLibrary|KKGetPath "EProjectSavedDir"))
  (bind _array (Utilities|Array|MakeArray _returnvalue "test.txt"))
  (bind _returnvalue_2 (Class|KKFileBlueprintFunctionLibrary|KKCombiePath _array))
  (Utilities|FlowControl|Sequence
    (:then_0
      (Development|PrintString _returnvalue_2)
      (Variables|Default|Setfile_path _returnvalue_2)
      (Development|PrintString (Utilities|String|Append "file exist ? " (Utilities|String|ToString(Boolean) (Class|KKFileBlueprintFunctionLibrary|KKFileExists _returnvalue_2)))))
    (:then_1
      (bind _returnvalue_3 (Class|KKFileBlueprintFunctionLibrary|KKSaveStringtoFile "this is a test string" (Variables|Default|Getfile_path)))
      (Development|PrintString (Utilities|String|Append "write string to file : " (Utilities|String|ToString(Boolean) _returnvalue_3))))
    (:then_2
      (Development|PrintString (Utilities|String|Append "load string to array : length -> " (Utilities|String|ToString(Integer) (Utilities|Array|Length (.Data (Class|KKFileBlueprintFunctionLibrary|KKLoadFiletoStringArray (Variables|Default|Getfile_path))))))))))

(fn ConstructionScript)